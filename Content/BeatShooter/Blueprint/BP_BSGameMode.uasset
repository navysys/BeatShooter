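; Game mode for BeatShooter that manages the menu flow and tracks score, combo, time and life.
; On BeginPlay it spawns title, mode-select and game-over widget actors, then switches screens by toggling their visibility and collision.
; Stat functions push values into WBP_Score, while StartGame and GameOver start and stop the Spawner.
; Life only drops in Challenge state, and reaching zero triggers game over with the final score.
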(event `self.ReceiveBeginPlay`
  (`self.InitUI`))

(fn `DecreaseLife`
  (bind _life (`self.Life`))
  (switch `/Game/BeatShooter/E_GameState` (`self.State`)
    (:`NewEnumerator1`
      (bind _result (`/Engine/EditorBlueprintResources/StandardMacros.DecrementInt` (`self.Life`))
        (:`  `
          (set `self.Life` _result)
          (bind _aswbp_score (cast `/Game/WBP_Score` (`WidgetComponent.GetWidget` (`/Game/BeatShooter/Blueprint/BP_WidgetActor.Widget` (`self.Widget_Score`)))))
          (set `/Game/WBP_Score.Life` _life _aswbp_score)
          (if (<= _life 0)
            (`self.GameOver`)))))))

(fn `GameOver`
  (`self.RunGameOverUI`)
  (`/Game/BeatShooter/Blueprint/BP_Spawner.EndSpawn` (`self.Spawner`)))

(fn `IncreaseCombo`
  (bind _result (`/Engine/EditorBlueprintResources/StandardMacros.IncrementInt` (`self.Combo`))
    (:`  `
      (set `self.Combo` _result)
      (bind _aswbp_score (cast `/Game/WBP_Score` (`WidgetComponent.GetWidget` (`/Game/BeatShooter/Blueprint/BP_WidgetActor.Widget` (`self.Widget_Score`)))))
      (set `/Game/WBP_Score.Combo` (`self.Combo`) _aswbp_score))))

(fn `IncreaseScoreInt`
  (bind _result (`/Engine/EditorBlueprintResources/StandardMacros.IncrementInt` (`self.ScoreInt`))
    (:`  `
      (set `self.ScoreInt` _result)
      (bind _aswbp_score (cast `/Game/WBP_Score` (`WidgetComponent.GetWidget` (`/Game/BeatShooter/Blueprint/BP_WidgetActor.Widget` (`self.Widget_Score`)))))
      (set `/Game/WBP_Score.Score` (`self.ScoreInt`) _aswbp_score))))

(fn `InitUI`
  (bind _returnvalue (`|SpawnActorFromClass` "/Game/BeatShooter/Blueprint/BP_TitleWidget.BP_TitleWidget_C" (`KismetMathLibrary.MakeTransform` (0.0 0.0 0.0)) "Undefined" "MultiplyWithRoot" null null))
  (set `self.Widget_Title` _returnvalue)
  (bind _returnvalue_2 (`|SpawnActorFromClass` "/Game/BeatShooter/Blueprint/BP_SelectModeWidget.BP_SelectModeWidget_C" (`KismetMathLibrary.MakeTransform` (0.0 0.0 0.0)) "Undefined" "MultiplyWithRoot" null null))
  (bind _output_get (set `self.Widget_SelectMode` _returnvalue_2))
  (bind _widget (`/Game/BeatShooter/Blueprint/BP_SelectModeWidget.Widget` _output_get))
  (`SceneComponent.SetVisibility` _widget false false)
  (`PrimitiveComponent.SetCollisionEnabled` _widget "NoCollision")
  (bind _returnvalue_3 (`|SpawnActorFromClass` "/Game/BeatShooter/Blueprint/BP_GameOverWidget.BP_GameOverWidget_C" (`KismetMathLibrary.MakeTransform` (0.0 0.0 0.0)) "Undefined" "MultiplyWithRoot" null null))
  (bind _output_get_2 (set `self.Widget_GameOver` _returnvalue_3))
  (bind _widget_2 (`/Game/BeatShooter/Blueprint/BP_GameOverWidget.Widget` _output_get_2))
  (`SceneComponent.SetVisibility` _widget_2 false false)
  (`PrimitiveComponent.SetCollisionEnabled` _widget_2 "NoCollision"))

(fn `ResetCombo`
  (set `self.Combo` 0)
  (bind _aswbp_score (cast `/Game/WBP_Score` (`WidgetComponent.GetWidget` (`/Game/BeatShooter/Blueprint/BP_WidgetActor.Widget` (`self.Widget_Score`)))))
  (set `/Game/WBP_Score.Combo` (`self.Combo`) _aswbp_score))

(fn `RunGameOverUI`
  (bind _widget_gameover (`self.Widget_GameOver`))
  (bind _aswbp_game_over (cast `/Game/WBP_GameOver` (`WidgetComponent.GetWidget` (`/Game/BeatShooter/Blueprint/BP_WidgetActor.Widget` (`self.Widget_GameOver`)))))
  (set `/Game/WBP_GameOver.Score` (`self.ScoreInt`) _aswbp_game_over)
  (`SceneComponent.SetVisibility` (`/Game/BeatShooter/Blueprint/BP_WidgetActor.Widget` _widget_gameover) true false)
  (`PrimitiveComponent.SetCollisionEnabled` (`/Game/BeatShooter/Blueprint/BP_WidgetActor.Widget` _widget_gameover) "QueryAndPhysics"))

(fn `RunSelectModeUI`
  (bind _widget_title (`self.Widget_Title`))
  (bind _widget_selectmode (`self.Widget_SelectMode`))
  (`SceneComponent.SetVisibility` (`/Game/BeatShooter/Blueprint/BP_WidgetActor.Widget` _widget_title) false false)
  (`PrimitiveComponent.SetCollisionEnabled` (`/Game/BeatShooter/Blueprint/BP_WidgetActor.Widget` _widget_title) "NoCollision")
  (`SceneComponent.SetVisibility` (`/Game/BeatShooter/Blueprint/BP_WidgetActor.Widget` _widget_selectmode) true false)
  (`PrimitiveComponent.SetCollisionEnabled` (`/Game/BeatShooter/Blueprint/BP_WidgetActor.Widget` _widget_selectmode) "QueryAndPhysics"))

(fn `RunTitleUI`
  (bind _widget_title (`self.Widget_Title`))
  (bind _widget_gameover (`self.Widget_GameOver`))
  (`SceneComponent.SetVisibility` (`/Game/BeatShooter/Blueprint/BP_WidgetActor.Widget` _widget_gameover) false false)
  (`PrimitiveComponent.SetCollisionEnabled` (`/Game/BeatShooter/Blueprint/BP_WidgetActor.Widget` _widget_gameover) "NoCollision")
  (`SceneComponent.SetVisibility` (`/Game/BeatShooter/Blueprint/BP_WidgetActor.Widget` _widget_title) true false)
  (`PrimitiveComponent.SetCollisionEnabled` (`/Game/BeatShooter/Blueprint/BP_WidgetActor.Widget` _widget_title) "QueryAndPhysics"))

(fn `SetScoreTime`
  (set `self.ScoreTime` (`/Game/BeatShooter/Blueprint/BP_Spawner.Time` (`self.Spawner`)))
  (bind _aswbp_score (cast `/Game/WBP_Score` (`WidgetComponent.GetWidget` (`/Game/BeatShooter/Blueprint/BP_WidgetActor.Widget` (`self.Widget_Score`)))))
  (set `/Game/WBP_Score.Time` (`KismetMathLibrary.FTrunc` (`self.ScoreTime`)) _aswbp_score))

(fn `StartGame`
  (bind _widget_selectmode (`self.Widget_SelectMode`))
  (`SceneComponent.SetVisibility` (`/Game/BeatShooter/Blueprint/BP_WidgetActor.Widget` _widget_selectmode) false false)
  (`PrimitiveComponent.SetCollisionEnabled` (`/Game/BeatShooter/Blueprint/BP_WidgetActor.Widget` _widget_selectmode) "NoCollision")
  (`/Game/BeatShooter/Blueprint/BP_Spawner.StartSpawn` (`self.Spawner`)))

(fn `UserConstructionScript`)