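; BP_Node is a moving note target in the BeatShooter game, meant to be shot while overlapping the Catcher.
; Tick moves it forward, easing to 75% of its initial speed; entering the Catcher swaps its material, quarters its speed and arms CurrentShoot.
; Bullet hits destroy it, flag the Spawner and report score and combo when armed, otherwise life loss and combo reset.
; Leaving the Catcher armed counts as a miss.
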(event `self.ReceiveBeginPlay`
  (set `self.Speed` (`self.InitSpeed`))
  (bind _asbp_bsgame_mode (cast `/Game/BeatShooter/Blueprint/BP_BSGameMode` (`GameplayStatics.GetGameMode`)))
  (bind _spawner (`/Game/BeatShooter/Blueprint/BP_BSGameMode.Spawner` _asbp_bsgame_mode))
  (set `self.Spawner` _spawner)
  (bind _catcher (`/Game/BeatShooter/Blueprint/BP_BSGameMode.Catcher` _asbp_bsgame_mode))
  (set `self.Catcher` _catcher)
  (bind _returnvalue_x (`KismetMathLibrary.BreakVector` (`self.K2_GetActorLocation` _spawner)))
  (bind _returnvalue_x_2 (`KismetMathLibrary.BreakVector` (`self.K2_GetActorLocation` _catcher)))
  (set `self.Distance` (- _returnvalue_x _returnvalue_x_2)))

(event `self.ReceiveTick`
  (params (DeltaSeconds :type "Float (single-precision)"))
  (bind _returnvalue_x (`KismetMathLibrary.BreakVector` (`self.K2_GetActorLocation`)))
  (bind _alpha (`self.Alpha`))
  (bind _returnvalue_x_2 (`KismetMathLibrary.BreakVector` (`self.K2_GetActorLocation` (`self.Catcher`))))
  (`|ExecutionSequence`
    (:`then_0`
      (if (> (- _returnvalue_x _returnvalue_x_2) 100.0)
        (if (<= _alpha 1.0)
          (bind _output_get (set `self.Alpha` (+ DeltaSeconds _alpha)))
          (set `self.Speed` (`KismetMathLibrary.Lerp` (`self.InitSpeed`) (* (`self.InitSpeed`) 0.75) _output_get)))))
    (:`then_1`
      (`self.K2_AddActorWorldOffset` (* (`self.GetActorForwardVector`) (* DeltaSeconds (`self.Speed`)))))))

(event `self.StaticMesh.OnComponentHit`
  (params (HitComponent :type "PrimitiveComponent Object Reference") (OtherActor :type "Actor Object Reference") (OtherComp :type "PrimitiveComponent Object Reference") (NormalImpulse :type "Vector Structure") (Hit :type "HitResult Structure (by ref)"))
  (bind _asbp_bullet (cast `/Game/BeatShooter/Blueprint/BP_Bullet` OtherActor))
  (set `/Game/BeatShooter/Blueprint/BP_Spawner.bIsNodeDestroy` true (`self.Spawner`))
  (bind _asbp_bsgame_mode (cast `/Game/BeatShooter/Blueprint/BP_BSGameMode` (`GameplayStatics.GetGameMode`)))
  (if (`self.bCurrentShoot`)
    (`/Game/BeatShooter/Blueprint/BP_BSGameMode.IncreaseScoreInt` _asbp_bsgame_mode)
    (`/Game/BeatShooter/Blueprint/BP_BSGameMode.IncreaseCombo` _asbp_bsgame_mode)
    (else
      (`/Game/BeatShooter/Blueprint/BP_BSGameMode.DecreaseLife` _asbp_bsgame_mode)
      (`/Game/BeatShooter/Blueprint/BP_BSGameMode.ResetCombo` _asbp_bsgame_mode)))
  (`self.K2_DestroyActor` _asbp_bullet)
  (set `self.bCurrentShoot` false)
  (`self.K2_DestroyActor`))

(event `self.StaticMesh.OnComponentBeginOverlap`
  (params (OverlappedComponent :type "PrimitiveComponent Object Reference") (OtherActor :type "Actor Object Reference") (OtherComp :type "PrimitiveComponent Object Reference") (OtherBodyIndex :type Integer) (bFromSweep :type Boolean) (SweepResult :type "HitResult Structure (by ref)"))
  (cast `/Game/BeatShooter/Blueprint/BP_Catcher` OtherActor)
  (set `self.bCurrentShoot` true)
  (`PrimitiveComponent.SetMaterial` (`self.StaticMesh`) 0 (`self.CurrentShootMaterial`))
  (set `self.Speed` (* (`self.Speed`) 0.25)))

(event `self.StaticMesh.OnComponentEndOverlap`
  (params (OverlappedComponent :type "PrimitiveComponent Object Reference") (OtherActor :type "Actor Object Reference") (OtherComp :type "PrimitiveComponent Object Reference") (OtherBodyIndex :type Integer))
  (cast `/Game/BeatShooter/Blueprint/BP_Catcher` OtherActor)
  (if (`self.bCurrentShoot`)
    (set `/Game/BeatShooter/Blueprint/BP_Spawner.bIsNodeDestroy` true (`self.Spawner`))
    (bind _asbp_bsgame_mode (cast `/Game/BeatShooter/Blueprint/BP_BSGameMode` (`GameplayStatics.GetGameMode`)))
    (`/Game/BeatShooter/Blueprint/BP_BSGameMode.DecreaseLife` _asbp_bsgame_mode)
    (`/Game/BeatShooter/Blueprint/BP_BSGameMode.ResetCombo` _asbp_bsgame_mode)
    (`self.K2_DestroyActor`)
    (else
      (`self.K2_DestroyActor`))))

(fn `UserConstructionScript`)