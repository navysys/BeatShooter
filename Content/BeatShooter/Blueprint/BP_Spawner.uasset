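; BP_Spawner spawns BP_Node targets for the beat shooter and registers itself with BP_BSGameMode.
; StartSpawn copies the game mode's state, then Tick advances a timer, calls SetScoreTime and runs that mode's spawn routine.
; Aim Training spawns a randomly placed node whenever one is destroyed, while Challenge spawns them at a shrinking interval down to a floor.
; Music loads data table rows and spawns nodes at their listed times and offsets.
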(event `self.ReceiveBeginPlay`
  (bind _asbp_bsgame_mode (cast `/Game/BeatShooter/Blueprint/BP_BSGameMode` (`GameplayStatics.GetGameMode`)))
  (set `/Game/BeatShooter/Blueprint/BP_BSGameMode.Spawner` self _asbp_bsgame_mode))

(event `self.ReceiveTick`
  (params (DeltaSeconds :type "Float (single-precision)"))
  (if (`self.bIsSpawnerStart`)
    (set `self.Time` (+ DeltaSeconds (`self.Time`)))
    (bind _asbp_bsgame_mode (cast `/Game/BeatShooter/Blueprint/BP_BSGameMode` (`GameplayStatics.GetGameMode`)))
    (`/Game/BeatShooter/Blueprint/BP_BSGameMode.SetScoreTime` _asbp_bsgame_mode)
    (switch `/Game/BeatShooter/E_GameState` (`self.GState`)
      (:`NewEnumerator0`
        (`self.SpawnToAfterDestroy`))
      (:`NewEnumerator1`
        (`self.SpawnToBecomeFaster`))
      (:`NewEnumerator2`
        (`self.SpawnToDatabase`)))))

(fn `EndSpawn`
  (set `self.bIsSpawnerStart` false))

(fn `InitDataTable`
  (bind _outrownames (`DataTableFunctionLibrary.GetDataTableRowNames` (`self.SpawnTable`)))
  (bind _output_get (set `self.Out Row Names` _outrownames))
  (for _array_element _output_get
    (bind _returnvalue (`|GetDataTableRow` "/Game/DT_SpawnTable.DT_SpawnTable" _array_element)
      (:`then`
        (`KismetArrayLibrary.Array_Add` (`self.Rows`) _returnvalue))))
  (set `self.NextSpawnTime` (`.Time_2_295B0050442B27255881AB9A55D27053` (break `/Game/ST_SpawnData` (`|GetArrayItem` (`self.Rows`)))))
  (set `self.DTLength` (`KismetArrayLibrary.Array_Length` (`self.Rows`))))

(fn `SpawnToAfterDestroy`
  (bind (_returnvalue_x _returnvalue_y _returnvalue_z) (`KismetMathLibrary.BreakVector` (`self.K2_GetActorLocation`)))
  (if (`self.bIsNodeDestroy`)
    (set `self.bIsNodeDestroy` false)
    (`|SpawnActorFromClass` "/Game/BeatShooter/Blueprint/BP_Node.BP_Node_C" (`KismetMathLibrary.MakeTransform` (`KismetMathLibrary.MakeVector` _returnvalue_x (+ _returnvalue_y (`KismetMathLibrary.RandomFloatInRange` -200.0 200.0)) (+ _returnvalue_z (`KismetMathLibrary.RandomFloatInRange` 20.0 200.0))) (struct :`Yaw` 180.0)) "Undefined" "MultiplyWithRoot" null 1500.0 null)))

(fn `SpawnToBecomeFaster`
  (bind (_returnvalue_x _returnvalue_y _returnvalue_z) (`KismetMathLibrary.BreakVector` (`self.K2_GetActorLocation`)))
  (bind _spawndelay (`self.SpawnDelay`))
  (if (> (- (`self.Time`) (`self.LastSpawnTime`)) (`self.SpawnDelay`))
    (`|SpawnActorFromClass` "/Game/BeatShooter/Blueprint/BP_Node.BP_Node_C" (`KismetMathLibrary.MakeTransform` (`KismetMathLibrary.MakeVector` _returnvalue_x (+ _returnvalue_y (`KismetMathLibrary.RandomFloatInRange` -200.0 200.0)) (+ _returnvalue_z (`KismetMathLibrary.RandomFloatInRange` 20.0 200.0))) (struct :`Yaw` 180.0)) "Undefined" "MultiplyWithRoot" null 600.0 null)
    (set `self.LastSpawnTime` (`self.Time`))
    (if (> _spawndelay 0.3)
      (set `self.SpawnDelay` (* _spawndelay 0.95)))))

(fn `SpawnToDatabase`
  (bind (_time _location) (break `/Game/ST_SpawnData` (`|GetArrayItem` (`self.Rows`) (`self.Count`))))
  (if (and (< (`self.NextSpawnTime`) (`self.Time`)) (not (`self.bIsSpawnComplete`)))
    (`|SpawnActorFromClass` "/Game/BeatShooter/Blueprint/BP_Node.BP_Node_C" (`KismetMathLibrary.MakeTransform` (+ (`self.K2_GetActorLocation`) _location) (struct :`Yaw` 180.0)) "Undefined" "MultiplyWithRoot" null 600.0 null)
    (bind _result (`/Engine/EditorBlueprintResources/StandardMacros.IncrementInt` (`self.Count`))
      (:`  `
        (if (>= _result (`self.DTLength`))
          (set `self.bIsSpawnComplete` true)
          (else
            (set `self.NextSpawnTime` _time)))))))

(fn `StartSpawn`
  (set `self.bIsSpawnerStart` true)
  (set `self.Time` 0.0)
  (bind _asbp_bsgame_mode (cast `/Game/BeatShooter/Blueprint/BP_BSGameMode` (`GameplayStatics.GetGameMode`)))
  (bind _output_get (set `self.GState` (`/Game/BeatShooter/Blueprint/BP_BSGameMode.State` _asbp_bsgame_mode)))
  (switch `/Game/BeatShooter/E_GameState` _output_get
    (:`NewEnumerator2`
      (`self.InitDataTable`))))

(fn `UserConstructionScript`)