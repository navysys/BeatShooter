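; BP_WidgetActor is a VR menu actor that keeps its widget near the camera and turned toward it.
; Each Tick rotates the widget to the camera, then moves it to camera location plus forward vector multiplied by (100,0,0), so the offset is only along world X.
; BeginPlay adds IMC_Menu and caches BP_BSVRPawn's left and right widget interaction components.
; Left and right interact actions press and release simulated left-mouse clicks through those components.
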(event `self.ReceiveBeginPlay`
  (`self.EnableInput` (`GameplayStatics.GetPlayerController` 0))
  (`EnhancedInputSubsystemInterface.AddMappingContext` (pcsubsystem `EnhancedInputLocalPlayerSubsystem` (`GameplayStatics.GetPlayerController` 0)) "/Game/VRTemplate/Input/IMC_Menu.IMC_Menu" 0 (struct))
  (bind _asbp_bsvrpawn (cast `/Game/BeatShooter/Blueprint/BP_BSVRPawn` (`GameplayStatics.GetPlayerPawn` 0)))
  (set `self.WidgetInteractionRefLeft` (`/Game/BeatShooter/Blueprint/BP_BSVRPawn.WidgetInteractionLeft` _asbp_bsvrpawn))
  (set `self.WidgetInteractionRefRight` (`/Game/BeatShooter/Blueprint/BP_BSVRPawn.WidgetInteractionRight` _asbp_bsvrpawn)))

(event `self.ReceiveTick`
  (params (DeltaSeconds :type "Float (single-precision)"))
  (bind _returnvalue (`GameplayStatics.GetPlayerCameraManager` 0))
  (bind _returnvalue_2 (`self.K2_GetActorLocation` _returnvalue))
  (`SceneComponent.K2_SetWorldRotation` (`self.Widget`) (`KismetMathLibrary.FindLookAtRotation` (`SceneComponent.K2_GetComponentLocation` (`self.Widget`)) _returnvalue_2) false false)
  (`SceneComponent.K2_SetWorldLocation` (`self.Widget`) (+ _returnvalue_2 (* (`SceneComponent.GetForwardVector` (`PlayerCameraManager.TransformComponent` _returnvalue)) (100.0 0.0 0.0))) false false))

(event `EnhancedInput|/Game/VRTemplate/Input/Actions/IA_Menu_Interact_Left`
  (params (ActionValue :type Boolean) (ElapsedSeconds :type "Float (double-precision)") (TriggeredSeconds :type "Float (double-precision)") (InputAction :type "InputAction Object Reference" :default "/Game/VRTemplate/Input/Actions/IA_Menu_Interact_Left.IA_Menu_Interact_Left"))
  (bind _widgetinteractionrefleft (`self.WidgetInteractionRefLeft`))
  (:`Started`
    (`WidgetInteractionComponent.PressPointerKey` _widgetinteractionrefleft "LeftMouseButton"))
  (:`Completed`
    (`WidgetInteractionComponent.ReleasePointerKey` _widgetinteractionrefleft "LeftMouseButton")))

(event `EnhancedInput|/Game/VRTemplate/Input/Actions/IA_Menu_Interact_Right`
  (params (ActionValue :type Boolean) (ElapsedSeconds :type "Float (double-precision)") (TriggeredSeconds :type "Float (double-precision)") (InputAction :type "InputAction Object Reference" :default "/Game/VRTemplate/Input/Actions/IA_Menu_Interact_Right.IA_Menu_Interact_Right"))
  (bind _widgetinteractionrefright (`self.WidgetInteractionRefRight`))
  (:`Started`
    (`WidgetInteractionComponent.PressPointerKey` _widgetinteractionrefright "LeftMouseButton"))
  (:`Completed`
    (`WidgetInteractionComponent.ReleasePointerKey` _widgetinteractionrefright "LeftMouseButton")))

(fn `UserConstructionScript`)