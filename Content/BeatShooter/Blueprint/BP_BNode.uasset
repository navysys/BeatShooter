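; BP_BNode is a moving target node in BeatShooter that travels along its forward vector each tick at Speed.
; Overlapping a BP_Catcher flags it as CurrentShoot, swaps its material and halves its speed; leaving the catcher clears the flag and destroys it.
; A hit from a BP_Bullet destroys both bullet and node, without checking the CurrentShoot flag.
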(event `self.ReceiveTick`
  (params (DeltaSeconds :type "Float (single-precision)"))
  (`self.K2_AddActorWorldOffset` (* (`self.GetActorForwardVector`) (* DeltaSeconds (`self.Speed`)))))

(event `self.StaticMesh.OnComponentHit`
  (params (HitComponent :type "PrimitiveComponent Object Reference") (OtherActor :type "Actor Object Reference") (OtherComp :type "PrimitiveComponent Object Reference") (NormalImpulse :type "Vector Structure") (Hit :type "HitResult Structure (by ref)"))
  (bind _asbp_bullet (cast `/Game/BeatShooter/Blueprint/BP_Bullet` OtherActor))
  (`self.K2_DestroyActor` _asbp_bullet)
  (`self.K2_DestroyActor`))

(event `self.StaticMesh.OnComponentBeginOverlap`
  (params (OverlappedComponent :type "PrimitiveComponent Object Reference") (OtherActor :type "Actor Object Reference") (OtherComp :type "PrimitiveComponent Object Reference") (OtherBodyIndex :type Integer) (bFromSweep :type Boolean) (SweepResult :type "HitResult Structure (by ref)"))
  (`|ExecutionSequence`
    (:`then_0`
      (cast `/Game/BeatShooter/Blueprint/BP_Catcher` OtherActor)
      (set `self.bCurrentShoot` true)
      (`PrimitiveComponent.SetMaterial` (`self.StaticMesh`) 0 (`self.CurrentShootMaterial`))
      (set `self.Speed` (* (`self.Speed`) 0.5)))))

(event `self.StaticMesh.OnComponentEndOverlap`
  (params (OverlappedComponent :type "PrimitiveComponent Object Reference") (OtherActor :type "Actor Object Reference") (OtherComp :type "PrimitiveComponent Object Reference") (OtherBodyIndex :type Integer))
  (cast `/Game/BeatShooter/Blueprint/BP_Catcher` OtherActor)
  (set `self.bCurrentShoot` false)
  (`self.K2_DestroyActor`))

(fn `UserConstructionScript`)